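; Locked door actor that opens when a player carrying at least one key enters its trigger box.
; On overlap it casts to PlayerCharacter, destroys the box so it fires once, and decrements the player's Keys count.
; The Cube mesh then snaps open with an instant local rotation and teleported offset rather than an animation.
; Debug prints show the remaining keys or a message that a key is needed.
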(event `self.Box.OnComponentBeginOverlap`
  (params (OverlappedComponent :type "PrimitiveComponent Object Reference") (OtherActor :type "Actor Object Reference") (OtherComp :type "PrimitiveComponent Object Reference") (OtherBodyIndex :type Integer) (bFromSweep :type Boolean) (SweepResult :type "HitResult Structure (by ref)"))
  (bind _cube (`self.Cube`))
  ;[1 1 1] Use key to open door
  (bind _asplayer_character (cast `/Game/Design/Robert/Character/PlayerCharacter` OtherActor))
  (bind _keys (`/Game/Design/Robert/Character/PlayerCharacter.Keys` _asplayer_character))
  (if (>= _keys 1)
    (`ActorComponent.K2_DestroyComponent` (`self.Box`))
    (bind _output_get (set `/Game/Design/Robert/Character/PlayerCharacter.Keys` (- _keys 1) _asplayer_character))
    (`KismetSystemLibrary.PrintString` (`KismetStringLibrary.Conv_IntToString` _output_get))
    (`SceneComponent.K2_AddLocalRotation` _cube (struct :`Yaw` 90.0) false false)
    (`SceneComponent.K2_AddLocalOffset` _cube (-100.0 -125.0 0.0) false true)
    (else
      (`KismetSystemLibrary.PrintString` "Need key to open door"))))

(fn `UserConstructionScript`)