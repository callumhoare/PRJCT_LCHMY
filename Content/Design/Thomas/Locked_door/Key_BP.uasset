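; Key_BP is a collectible key pickup, stored with a locked-door design.
; When a PlayerCharacter overlaps its Box, it destroys its Cube, Box and PointLight components, leaving the actor itself in place.
; It then increments the player's HotkeysPerRow variable, which appears to serve as the key count despite its name, and prints the new value as a string.
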(event `self.Box.OnComponentBeginOverlap`
  (params (OverlappedComponent :type "PrimitiveComponent Object Reference") (OtherActor :type "Actor Object Reference") (OtherComp :type "PrimitiveComponent Object Reference") (OtherBodyIndex :type Integer) (bFromSweep :type Boolean) (SweepResult :type "HitResult Structure (by ref)"))
  ;[1 1 1] Collect Key
  (bind _asplayer_character (cast `/Game/Design/Robert/Character/PlayerCharacter` OtherActor))
  (`ActorComponent.K2_DestroyComponent` (`self.Cube`))
  (`ActorComponent.K2_DestroyComponent` (`self.Box`))
  (`ActorComponent.K2_DestroyComponent` (`self.PointLight`))
  (bind _output_get (set `/Game/Design/Robert/Character/PlayerCharacter.HotkeysPerRow` (+ (`/Game/Design/Robert/Character/PlayerCharacter.HotkeysPerRow` _asplayer_character) 1) _asplayer_character))
  (`KismetSystemLibrary.PrintString` (`KismetStringLibrary.Conv_IntToString` _output_get)))

(fn `UserConstructionScript`)