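; Speed potion pickup that temporarily boosts the player character's walk speed.
; When a PlayerCharacter overlaps the Box, it shows an ActiveSpeed widget and destroys its Cube and Box components, leaving the actor alive to run the timer.
; It raises player 0's MaxWalkSpeed, then after a Delay sets it to a hard-coded lower value and calls RemoveAllWidgets, which clears every widget, not just its own.
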(event `self.Box.OnComponentBeginOverlap`
  (params (OverlappedComponent :type "PrimitiveComponent Object Reference") (OtherActor :type "Actor Object Reference") (OtherComp :type "PrimitiveComponent Object Reference") (OtherBodyIndex :type Integer) (bFromSweep :type Boolean) (SweepResult :type "HitResult Structure (by ref)"))
  (bind _charactermovement (`Character.CharacterMovement` (cast `/Game/Design/Robert/Character/PlayerCharacter` (`GameplayStatics.GetPlayerCharacter` 0) :!pure true)))
  (cast `/Game/Design/Robert/Character/PlayerCharacter` OtherActor)
  (bind _returnvalue (`|CreateWidget` "/Game/Design/Thomas/Wind_Obstacle/Blueprints/ActiveSpeed.ActiveSpeed_C"))
  (`UserWidget.AddToViewport` _returnvalue 0)
  (`ActorComponent.K2_DestroyComponent` (`self.Cube`))
  (`ActorComponent.K2_DestroyComponent` (`self.Box`))
  (set `CharacterMovementComponent.MaxWalkSpeed` 1250.0 _charactermovement)
  (`KismetSystemLibrary.Delay` 9.0)
  (set `CharacterMovementComponent.MaxWalkSpeed` 1000.0 _charactermovement)
  (`WidgetLayoutLibrary.RemoveAllWidgets`))

(fn `UserConstructionScript`)